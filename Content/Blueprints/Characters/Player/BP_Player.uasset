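; Player character Blueprint that provides switching between locked and free camera orientation.
; LockCameraOrientation makes the character follow controller yaw, while FreeCameraOrientation makes it rotate toward movement, by toggling controller yaw and the movement component's orient-to-movement flag.
; BeginPlay only calls the parent, and an unconnected node would play a melee attack montage from a randomly chosen section.
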(event `self.ReceiveBeginPlay`
  (`parent.ReceiveBeginPlay`))

(fn `FreeCameraOrientation`
  (`|ExecutionSequence`
    (:`then_0`
      (set `self.bUseControllerRotationYaw` false))
    (:`then_1`
      (set `CharacterMovementComponent.bOrientRotationToMovement` true (`self.CharacterMovement`)))))

(fn `LockCameraOrientation`
  (`|ExecutionSequence`
    (:`then_0`
      (set `self.bUseControllerRotationYaw` true))
    (:`then_1`
      (set `CharacterMovementComponent.bOrientRotationToMovement` false (`self.CharacterMovement`)))))

(fn `UserConstructionScript`
  (`parent.UserConstructionScript`))