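; BP_PlayerController is the player controller that routes movement, look, jump and melee attack input to the BP_Player pawn.
; It caches the controlled pawn on BeginPlay, then applies movement along the camera's forward and right vectors, scaled by MoveValue.
; Turn adds yaw directly, while LookUp adds pitch only when the predicted control rotation stays within a wrapped angle range, limiting vertical look.
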(event `self.ReceiveBeginPlay`
  (bind _asbp_player (cast `/Game/Blueprints/Characters/Player/BP_Player` (`self.K2_GetPawn`)))
  (set `self.PlayerRef` _asbp_player))

(event `InputAxis|MoveForward`
  (params (AxisValue :type "Float (single-precision)"))
  (bind _playerref (`self.PlayerRef`))
  ;[1 1 1] Movement Control
  (`Pawn.AddMovementInput` _playerref (`SceneComponent.GetForwardVector` (`/Game/Blueprints/Characters/Player/BP_Player.Camera` _playerref)) (* AxisValue (`self.MoveValue`)) false))

(event `InputAction|Jump`
  (params (Key :type "Key Structure"))
  ;[1 1 1] Movement Control
  (:`Pressed`
    (`Character.Jump` (`self.PlayerRef`))))

(event `Key|LeftMouseButton`
  (params (Key :type "Key Structure"))
  (:`Pressed`
    (`/Game/Blueprints/Characters/BP_BaseCharacter.MeleeAttack` (`self.PlayerRef`))))

(event `InputAxis|Turn`
  (params (AxisValue :type "Float (single-precision)"))
  ;[1 1 1] Movement Control
  (`self.AddYawInput` AxisValue))

(event `InputAxis|MoveRight`
  (params (AxisValue :type "Float (single-precision)"))
  (bind _playerref (`self.PlayerRef`))
  ;[1 1 1] Movement Control
  (`Pawn.AddMovementInput` _playerref (`SceneComponent.GetRightVector` (`/Game/Blueprints/Characters/Player/BP_Player.Camera` _playerref)) (* AxisValue (`self.MoveValue`)) false))

(event `InputAxis|LookUp`
  (params (AxisValue :type "Float (single-precision)"))
  (bind (_returnvalue_roll _returnvalue_pitch) (`KismetMathLibrary.BreakRotator` (`self.GetControlRotation`)))
  (bind _returnvalue (+ (* AxisValue (`self.GetDeprecatedInputPitchScale`)) _returnvalue_pitch))
  ;[1 1 1] Movement Control
  (if (or (and (> _returnvalue 300.0) (<= _returnvalue 999.0)) (and (>= _returnvalue -999.0) (< _returnvalue 45.0)))
    (`self.AddPitchInput` AxisValue)))

(fn `UserConstructionScript`)